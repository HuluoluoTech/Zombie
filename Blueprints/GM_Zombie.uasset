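; GM_Zombie is the game mode for a wave-based zombie shooter.
; Each wave spawns an ammo pickup at a random listed location and four zombies per wave number, split between two spawn points.
; ZombieKilled counts down the survivors; clearing a wave increments it, shows the wave UI on the first-person character and spawns the next after a delay.
; Clearing MaxWave shows the win UI instead.
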(event `self.ReceiveBeginPlay`
  (`self.StartGame`))

(event `StartGame`
  (`self.SpawnZombies`))

(event `SpawnZombies`
  ;[1 1 1] 每个wave创建zombie
  (`self.SpwanAmmo`)
  (bind _output_get (set `self.ZombieTotal` (* (`self.CurrentWave`) 4)))
  (set `self.ZombieLeft` _output_get)
  (for _index (range (`self.ZombieTotal`))
    (if (== _index (/ (`self.ZombieLeft`) 2))
      (break)
      (else
        (`|SpawnActorFromClass` "/Game/_Main/Zombie/BP_Zombie.BP_Zombie_C" (`self.SpawnLocation1`) "Undefined" "OverrideRootScale" null null))))
  (for _ (range (/ (`self.ZombieTotal`) 2))
    (`|SpawnActorFromClass` "/Game/_Main/Zombie/BP_Zombie.BP_Zombie_C" (`self.SpawnLocation2`) "Undefined" "OverrideRootScale" null null)))

(event `ZombieKilled`
  ;[1 1 1] 当前wave的zombie死完了
  (bind _result (`/Engine/EditorBlueprintResources/StandardMacros.DecrementInt` (`self.ZombieLeft`))
    (:`  `
      (if (<= _result 0)
        (`self.WaveInc`)))))

(event `WaveInc`
  ;[1 1 1] wave 增加
  (if (== (`self.CurrentWave`) (`self.MaxWave`))
    (`self.PlayerWins`)
    (else
      (`/Engine/EditorBlueprintResources/StandardMacros.IncrementInt` (`self.CurrentWave`)
        (:`  `
          (`self.WaveStart`))))))

(event `WaveStart`
  ;[1 1 1] waveStart Event
  (bind _asbp_first_person_character (cast `/Game/_Main/Blueprints/BP_FirstPersonCharacter` (`GameplayStatics.GetPlayerCharacter` 0)))
  (`/Game/_Main/Blueprints/BP_FirstPersonCharacter.ShowWidgetUI` _asbp_first_person_character (`self.CurrentWave`))
  (`KismetSystemLibrary.Delay` 3.0)
  (`self.SpawnZombies`))

(event `PlayerWins`
  ;[1 1 1] Player 胜利
  (bind _asbp_first_person_character (cast `/Game/_Main/Blueprints/BP_FirstPersonCharacter` (`GameplayStatics.GetPlayerCharacter` 0)))
  (`/Game/_Main/Blueprints/BP_FirstPersonCharacter.showWinUI` _asbp_first_person_character))

(event `SpwanAmmo`
  ;[1 1 1] 创建弹夹
  (`|SpawnActorFromClass` "/Game/_Main/Blueprints/BP_AmmoPickup.BP_AmmoPickup_C" (`KismetMathLibrary.MakeTransform` (`|GetArrayItem` (`self.AmmoCrateLocations`) (`KismetMathLibrary.RandomInteger` 3))) "Undefined" "OverrideRootScale" null null))

(fn `UserConstructionScript`)